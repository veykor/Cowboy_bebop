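; Projectile actor that flies flat across the level and explodes when it overlaps anything other than a Character.
; Tick moves it along a 2D Direction scaled by Speed and delta time, pinning world Z to a fixed height.
; Overlap spawns a small explosion with a 2D sound and destroys only the Sphere component.
; The actor itself is removed by a timer started on BeginPlay.
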(event Custom|destroyme
  (Actor|DestroyActor))

(event EventBeginPlay
  (Utilities|Time|SetTimerbyEvent (delegate Custom|destroyme) 3.0))

(event Collision|EventActorBeginOverlap
  (params (OtherActor :type Actor%20Object%20Reference))
  (bind _sphere (Variables|Default|GetSphere))
  (Utilities|Casting|CastToCharacter OtherActor
    (:CastFailed
      (Effects|SpawnEmitteratLocation "/Game/StarterContent/Particles/P_Explosion.P_Explosion" (Transformation|GetActorLocation) "0, 0, 0" "0.200000,0.200000,0.200000")
      (Audio|PlaySound2D "/Game/StarterContent/Audio/Explosion01.Explosion01" 1.0 1.0 0.0 0 0)
      (Utilities|IsValid _sphere
        (:Is%20Valid
          (Components|DestroyComponent _sphere))))))

(event EventTick
  (params (DeltaSeconds :type Float%20%28single-precision%29))
  (bind _returnvalue (Transformation|GetActorLocation))
  (bind _direction (Variables|Default|Getdirection))
  (bind _speed (Variables|Default|Getspeed))
  (bind _returnvalue_2 (* DeltaSeconds _speed _direction))
  (bind _returnvalue_3 (Math|Conversions|ToVector(Vector2D) _returnvalue_2))
  (bind _returnvalue_4 (+ _returnvalue_3 _returnvalue))
  (Transformation|SetActorLocation (Math|Vector|MakeVector (.x _returnvalue_4) (.y _returnvalue_4) 1e+01) false false))

(fn ConstructionScript)