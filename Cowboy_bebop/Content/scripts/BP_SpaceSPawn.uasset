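; BP_SpaceSPawn is a player-controlled space pawn with Enhanced Input movement and a placeholder fire action.
; BeginPlay adds the input mapping context for its player controller, then sets a starting location and rotation.
; The move action stores a 2D value, cleared on release or cancel, which Tick applies along the actor's right and forward vectors, scaled by speed and delta time, without sweeping.
; Fire and Tick print debug strings.
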(event Input|EnhancedActionEvents|EnhancedInputActionBPInputFire
  (params (ActionValue :type Boolean) (ElapsedSeconds :type Float%20%28double-precision%29) (TriggeredSeconds :type Float%20%28double-precision%29) (InputAction :type Input%20Action%20Object%20Reference :default "/Game/scripts/BPInputFire.BPInputFire"))
  (:Started
    (Development|PrintString "Fire")))

(event Input|EnhancedActionEvents|EnhancedInputActionBP_InputMove
  (params (ActionValue :type Vector%202D%20Structure) (ElapsedSeconds :type Float%20%28double-precision%29) (TriggeredSeconds :type Float%20%28double-precision%29) (InputAction :type Input%20Action%20Object%20Reference :default "/Game/scripts/BP_InputMove.BP_InputMove"))
  (:Triggered
    (Variables|Default|SetmoveVal ActionValue))
  (:Canceled
    (Variables|Default|SetmoveVal "" :!label _label))
  (:Completed
    (goto _label)))

(event EventBeginPlay
  (bind _asplayer_controller (Utilities|Casting|CastToPlayerController (Pawn|GetController)))
  (Utilities|IsValid (PlayerController|LocalPlayerSubsystems|GetEnhancedInputLocalPlayerSubsystem _asplayer_controller)
    (:Is%20Valid
      (Input|AddMappingContext (PlayerController|LocalPlayerSubsystems|GetEnhancedInputLocalPlayerSubsystem _asplayer_controller) "/Game/scripts/BPInputMapping.BPInputMapping" 0 "(bIgnoreAllPressedKeysUntilRelease=True,bForceImmediately=False,bNotifyUserSettings=False)")
      (Transformation|SetActorLocationAndRotation "0, 0, 0" "0.000000,90.000000,0.000000"))))

(event Collision|EventActorBeginOverlap
  (params (OtherActor :type Actor%20Object%20Reference)))

(event EventTick
  (params (DeltaSeconds :type Float%20%28single-precision%29))
  (bind _returnvalue (Transformation|GetActorLocation))
  (bind _returnvalue_2 (Transformation|GetActorForwardVector))
  (bind _returnvalue_3 (Transformation|GetActorRightVector))
  (bind _speed (Variables|Default|Getspeed))
  (bind _moveval (Variables|Default|GetmoveVal))
  (bind _returnvalue_4 (* (.y _moveval) _returnvalue_2))
  (bind _returnvalue_5 (* _returnvalue_3 (.x _moveval)))
  (bind _returnvalue_6 (+ _returnvalue_5 _returnvalue_4))
  (bind _returnvalue_7 (* DeltaSeconds _speed _returnvalue_6))
  (bind _returnvalue_8 (+ _returnvalue_7 _returnvalue))
  (Development|PrintString (Utilities|String|ToString(Vector) _returnvalue_8))
  (Transformation|SetActorLocation _returnvalue_8 false false))

(fn ConstructionScript)