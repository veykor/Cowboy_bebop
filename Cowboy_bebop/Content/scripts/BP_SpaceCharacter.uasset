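; Player-controlled space character that flies with inertia and fires projectiles, using Enhanced Input.
; Tick eases a movement vector toward the input through an inertia integrator, then moves the actor along its right and forward axes, banking with lateral motion at a fixed yaw.
; Fire input spawns a projectile ahead of the actor, with a timer-reset flag limiting the fire rate.
; Overlaps only print the other actor's name.
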(event Custom|fireDelay
  (Variables|Default|SetenableFire true))

(event Input|EnhancedActionEvents|EnhancedInputActionBP_InputMove
  (params (ActionValue :type Vector%202D%20Structure) (ElapsedSeconds :type Float%20%28double-precision%29) (TriggeredSeconds :type Float%20%28double-precision%29) (InputAction :type Input%20Action%20Object%20Reference :default "/Game/scripts/BP_InputMove.BP_InputMove"))
  (:Triggered
    (Variables|Default|SetmoveVal ActionValue))
  (:Canceled
    (Variables|Default|SetmoveVal "" :!label _label))
  (:Completed
    (goto _label)))

(event Input|EnhancedActionEvents|EnhancedInputActionBPInputFire
  (params (ActionValue :type Boolean) (ElapsedSeconds :type Float%20%28double-precision%29) (TriggeredSeconds :type Float%20%28double-precision%29) (InputAction :type Input%20Action%20Object%20Reference :default "/Game/scripts/BPInputFire.BPInputFire"))
  (if (Variables|Default|GetenableFire)
    (CallFunction|Shot (Variables|Default|GetproyectilPrefab))
    (Variables|Default|SetenableFire false)
    (Utilities|Time|SetTimerbyEvent (delegate Custom|fireDelay) (Variables|Default|GettimeBetweenFire))))

(event EventBeginPlay
  (bind _asplayer_controller (Utilities|Casting|CastToPlayerController (Pawn|GetController)))
  (Utilities|IsValid (PlayerController|LocalPlayerSubsystems|GetEnhancedInputLocalPlayerSubsystem _asplayer_controller)
    (:Is%20Valid
      (Input|AddMappingContext (PlayerController|LocalPlayerSubsystems|GetEnhancedInputLocalPlayerSubsystem _asplayer_controller) "/Game/scripts/BPInputMapping.BPInputMapping" 0 "(bIgnoreAllPressedKeysUntilRelease=True,bForceImmediately=False,bNotifyUserSettings=False)"))))

(event Collision|EventActorBeginOverlap
  (params (OtherActor :type Actor%20Object%20Reference))
  (Development|PrintString (Utilities|GetDisplayName OtherActor)))

(event EventTick
  (params (DeltaSeconds :type Float%20%28single-precision%29))
  (bind _output_get (Variables|Default|Setintegrator (+ (stale _output_get) (* (Variables|Default|GetinertiaFactor) DeltaSeconds (- (Variables|Default|GetmoveVal) (stale _output_get))))))
  (Transformation|SetActorLocationAndRotation (+ (* DeltaSeconds (Variables|Default|Getspeed) (+ (* (Transformation|GetActorRightVector) (.x (Variables|Default|Getintegrator))) (* (.y (Variables|Default|Getintegrator)) (Transformation|GetActorForwardVector)))) (Transformation|GetActorLocation)) (Math|Rotator|MakeRotator (* (.x (Variables|Default|Getintegrator)) 45.0) 0.0 9e+01)))

(fn ConstructionScript)

(fn Shot
  (params (proyectilPrefab :type Actor%20Class%20Reference))
  (Game|SpawnActorfromClass proyectilPrefab (Math|Transform|MakeTransform (+ (Transformation|GetActorLocation) (* (Transformation|GetActorForwardVector) (Variables|Default|GetproyectilOffset))) "0, 0, 0" "1.000000,1.000000,1.000000") "Undefined" "MultiplyWithRoot" 0 0))